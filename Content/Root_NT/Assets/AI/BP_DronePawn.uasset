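; BP_DronePawn is a drone pawn that patrols back and forth between its spawn location and a relative offset point.
; Tick moves it by a fixed per-frame step, unscaled by delta time and without sweep.
; Within a near distance, a DoOnce-gated delay pauses it, then a FlipFlop reverses the destination.
; A trigger overlap with Core_PlayerCharacter only prints a red "DETECTED" message.
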(event OnComponentBeginOverlap(Trigger)
  (params (OverlappedComponent :type Primitive%20Component%20Object%20Reference) (OtherActor :type Actor%20Object%20Reference) (OtherComp :type Primitive%20Component%20Object%20Reference) (OtherBodyIndex :type Integer) (bFromSweep :type Boolean) (SweepResult :type Hit%20Result%20Structure%20%28by%20ref%29))
  ;[1 1 1] Detection
  (Utilities|Casting|CastToCore_PlayerCharacter OtherActor)
  (Development|PrintString "DETECTED" true true "(R=1.000000,G=0.088542,B=0.088542,A=1.000000)"))

(event EventBeginPlay
  (bind _returnvalue (Transformation|GetActorLocation))
  ;[1 1 1] Saving start and target positions
  (Variables|Default|SetWorldPos1 (+ (Variables|Default|GetPos1) _returnvalue))
  (Variables|Default|SetStartPos _returnvalue))

(event EventTick
  (params (DeltaSeconds :type Float%20%28single-precision%29))
  ;[1 1 1] Moving to position (either start or target positions)
  (if (>= (Math|Vector|VectorLength (select (Variables|Default|GetMovingToStart) (- (Transformation|GetActorLocation) (Variables|Default|GetStartPos)) (- (Transformation|GetActorLocation) (Variables|Default|GetWorldPos1)))) (Variables|Default|GetMinNearDistance))
    (Transformation|AddActorWorldOffset (* (select (Variables|Default|GetMovingToStart) (Math|Vector|Normalize (- (Variables|Default|GetStartPos) (Transformation|GetActorLocation))) (Math|Vector|Normalize (- (Variables|Default|GetWorldPos1) (Transformation|GetActorLocation)))) (Variables|Default|GetSpeed)))
    (else
      ;[1 1 1] Stop and turn
      (Utilities|FlowControl|DoOnce false :!label _label
        (:Completed
          (Utilities|FlowControl|Delay (Variables|Default|GetStopDuration))
          (Utilities|FlowControl|FlipFlop
            (:A
              (Variables|Default|SetMovingToStart true)
              (goto _label Reset))
            (:B
              (Variables|Default|SetMovingToStart false)
              (goto _label Reset))))))))

(fn ConstructionScript)