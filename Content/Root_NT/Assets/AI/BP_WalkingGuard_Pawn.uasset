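; BP_WalkingGuard_Pawn is a guard pawn that moves its Cube component along the WalkPath spline in a repeating one-way loop.
; Each tick advances the distance at constant Speed with FInterpToConstant, then sets the cube's world location and rotation from the spline, sampling rotation in local space.
; Reaching the end resets a DoOnce, so the next tick snaps the distance back to the start.
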(event EventTick
  (params (DeltaSeconds :type Float%20%28single-precision%29))
  (Utilities|FlowControl|Sequence
    (:then_0
      (Utilities|FlowControl|DoOnce false :!label _label
        (:Completed
          (Variables|Default|SetCurrentDistanceAlongSpline 0.0))))
    (:then_1
      (bind _output_get (Variables|Default|SetCurrentDistanceAlongSpline (Math|Interpolation|FInterptoConstant (Variables|Default|GetCurrentDistanceAlongSpline) (Spline|GetSplineLength (Variables|Default|GetWalkPath)) DeltaSeconds (Variables|Default|GetSpeed))))
      (Transformation|SetWorldLocation (Variables|Default|GetCube) (Spline|GetLocationatDistanceAlongSpline (Variables|Default|GetWalkPath) _output_get "World") false false)
      (Transformation|SetWorldRotation (Variables|Default|GetCube) (Spline|GetRotationatDistanceAlongSpline (Variables|Default|GetWalkPath) _output_get "Local") false false)
      (if (>= (Variables|Default|GetCurrentDistanceAlongSpline) (Spline|GetSplineLength (Variables|Default|GetWalkPath)))
        (goto _label Reset)))))

(fn ConstructionScript)