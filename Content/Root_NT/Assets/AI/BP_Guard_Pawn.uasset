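; Guard pawn that, once StartWalking is called, moves its Cube along the WalkPath spline toward the end at constant speed.
; Tick advances the distance along the spline with FInterpToConstant, then sets the Cube's location from world-space and rotation from local-space spline samples.
; A TextRender label is hidden at BeginPlay, shown when walking starts, and held at a fixed world rotation each walking tick.
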(event Custom|Start%20Walking
  (Variables|Default|SetisWalking true)
  (Rendering|SetVisibility (Variables|Default|GetTextRender) true false))

(event EventTick
  (params (DeltaSeconds :type Float%20%28single-precision%29))
  (if (Variables|Default|GetisWalking)
    (bind _output_get (Variables|Default|SetCurrentDistanceAlongSpline (Math|Interpolation|FInterptoConstant (Variables|Default|GetCurrentDistanceAlongSpline) (Spline|GetSplineLength (Variables|Default|GetWalkPath)) DeltaSeconds (Variables|Default|GetSpeed))))
    (Transformation|SetWorldLocation (Variables|Default|GetCube) (Spline|GetLocationatDistanceAlongSpline (Variables|Default|GetWalkPath) _output_get "World") false false)
    (Transformation|SetWorldRotation (Variables|Default|GetCube) (Spline|GetRotationatDistanceAlongSpline (Variables|Default|GetWalkPath) _output_get "Local") false false)
    (Transformation|SetWorldRotation (Variables|Default|GetTextRender) "45.000000,180.000000, 0" false false)))

(event EventBeginPlay
  (Rendering|SetVisibility (Variables|Default|GetTextRender) false false))

(fn ConstructionScript)