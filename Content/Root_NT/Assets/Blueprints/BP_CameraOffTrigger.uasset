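; BP_CameraOffTrigger is an interaction volume that lets the player shut off the game's cameras.
; Overlapping the trigger as a Core_PlayerCharacter enables input on the actor, and leaving it disables input again.
; While input is enabled, pressing E calls TurnOffCameras on Core_GameInstance, gated by a DoOnce so it fires a single time.
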(event OnComponentBeginOverlap(Trigger)
  (params (OverlappedComponent :type Primitive%20Component%20Object%20Reference) (OtherActor :type Actor%20Object%20Reference) (OtherComp :type Primitive%20Component%20Object%20Reference) (OtherBodyIndex :type Integer) (bFromSweep :type Boolean) (SweepResult :type Hit%20Result%20Structure%20%28by%20ref%29))
  (Utilities|Casting|CastToCore_PlayerCharacter OtherActor)
  (Input|EnableInput (Game|GetPlayerController 0)))

(event OnComponentEndOverlap(Trigger)
  (params (OverlappedComponent :type Primitive%20Component%20Object%20Reference) (OtherActor :type Actor%20Object%20Reference) (OtherComp :type Primitive%20Component%20Object%20Reference) (OtherBodyIndex :type Integer))
  (Utilities|Casting|CastToCore_PlayerCharacter OtherActor)
  (Input|DisableInput (Game|GetPlayerController 0)))

(event Input|ActionEvents|InputActionE
  (params (Key :type Key%20Structure))
  (:Pressed
    (Utilities|FlowControl|DoOnce false
      (:Completed
        (bind _ascore_game_instance (Utilities|Casting|CastToCore_GameInstance (Game|GetGameInstance)))
        (Default|TurnOffCameras _ascore_game_instance)))))

(fn ConstructionScript)