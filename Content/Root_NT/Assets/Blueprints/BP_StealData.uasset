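; BP_StealData is a one-time interactable that lets the player steal data, triggering a scripted guard response.
; Its trigger volume enables E-key input while the player character overlaps it.
; Pressing E shows the data text, then starts one guard walking and sends the listening guards to the data room.
; A delay-timed sequence then briefly halts those guards while OpenText shows, resumes them and opens the door.
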(event OnComponentBeginOverlap(Trigger)
  (params (OverlappedComponent :type Primitive%20Component%20Object%20Reference) (OtherActor :type Actor%20Object%20Reference) (OtherComp :type Primitive%20Component%20Object%20Reference) (OtherBodyIndex :type Integer) (bFromSweep :type Boolean) (SweepResult :type Hit%20Result%20Structure%20%28by%20ref%29))
  (Utilities|Casting|CastToCore_PlayerCharacter OtherActor)
  (Input|EnableInput (Game|GetPlayerController 0)))

(event OnComponentEndOverlap(Trigger)
  (params (OverlappedComponent :type Primitive%20Component%20Object%20Reference) (OtherActor :type Actor%20Object%20Reference) (OtherComp :type Primitive%20Component%20Object%20Reference) (OtherBodyIndex :type Integer))
  (Utilities|Casting|CastToCore_PlayerCharacter OtherActor)
  (Input|DisableInput (Game|GetPlayerController 0)))

(event EventBeginPlay
  (Rendering|SetVisibility (Variables|Default|GetDataText) false false)
  (Rendering|SetVisibility (Variables|Default|GetOpenText) false false))

(event Input|ActionEvents|InputActionE
  (params (Key :type Key%20Structure))
  (:Pressed
    (Utilities|FlowControl|DoOnce false
      (:Completed
        (Rendering|SetVisibility (Variables|Default|GetDataText) true false)
        (Utilities|FlowControl|Delay 1.0)
        (Utilities|FlowControl|Sequence
          (:then_0
            (Default|StartWalking (Variables|Default|GetThatOneGuard)))
          (:then_1
            (for _array_element (Variables|Default|GetListeningGuards)
              (Default|WalktoDataRoom _array_element))
            (Utilities|FlowControl|Delay 2.5)
            (Rendering|ToggleVisibility (Variables|Default|GetOpenText) false)
            (for _array_element_2 (Variables|Default|GetListeningGuards)
              (Variables|/Game/Root_NT/Assets/AI/BP_TriggeredGuard_Pawn.BP_TriggeredGuard_Pawn_C|SetSpeed _array_element_2 0.0))
            (Utilities|FlowControl|Delay 2.0)
            (for _array_element_3 (Variables|Default|GetListeningGuards)
              (Variables|/Game/Root_NT/Assets/AI/BP_TriggeredGuard_Pawn.BP_TriggeredGuard_Pawn_C|SetSpeed _array_element_3 1.5e+02))
            (Default|Open (Variables|Default|GetDoor))
            (Rendering|ToggleVisibility (Variables|Default|GetOpenText) false)))))))

(fn ConstructionScript)