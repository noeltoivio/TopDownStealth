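; BP_Camera is a camera prop with a spotlight that can sweep back and forth between its starting rotation and a target rotation.
; If movement is enabled, a speed-scaled timeline lerps the actor's rotation, with a delay chained off its Update pin.
; After that delay, a FlipFlop sets the sweep direction and MoveCamera calls itself to replay the timeline.
; TurnOff stops the timeline, tilts the mesh, hides the spotlight and blocks further sweeps.
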(event Custom|Move%20Camera
  ;[1 1 1] Moving to position (either start or target positions)
  (if (not (Variables|Default|GetisOff))
    (bind _newtrack_0 (Timeline|Rotate%20Timeline PlayFromStart)
      (:Update
        (Transformation|SetActorRotation (select (Variables|Default|GetRotationgToStart) (Math|Rotator|Lerp(Rotator) (Variables|Default|GetTargetRot) (Variables|Default|GetStartRot) _newtrack_0) (Math|Rotator|Lerp(Rotator) (Variables|Default|GetStartRot) (Variables|Default|GetTargetRot) _newtrack_0)))
        (Utilities|FlowControl|Delay (Variables|Default|GetPauseDelay))
        (Utilities|FlowControl|FlipFlop
          (:A
            (Variables|Default|SetRotationgToStart true))
          (:B
            (Variables|Default|SetRotationgToStart false)))
        (CallFunction|MoveCamera)))))

(event Custom|Turn%20Off
  (Audio|Components|Audio|Stop (Variables|Default|GetRotate%20Timeline))
  (Transformation|AddLocalRotation (Variables|Default|GetSM_Camera) "30.000000, 0, 0" false false)
  (Rendering|SetVisibility (Variables|Default|GetSpotLight) false false)
  (Variables|Default|SetisOff true))

(event EventBeginPlay
  ;[1 1 1] Saving start and target positions
  (Variables|Default|SetStartRot (Transformation|GetActorRotation))
  (if (Variables|Default|GetWillMove)
    (CallFunction|MoveCamera)
    (Components|Timeline|SetPlayRate (Variables|Default|GetRotate%20Timeline) (Variables|Default|GetRotationSpeedMutiplier))))

(fn ConstructionScript)