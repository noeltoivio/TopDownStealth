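; BP_SplineDronePawn is a drone that flies a looping route along its TravelPath spline and detects the player.
; Tick advances the distance along the spline at constant Speed, moves and rotates the StaticMesh to that point, then restarts from zero at the end.
; Location is sampled in world space, while rotation is sampled in local space but applied as world rotation.
; A Trigger overlap with Core_PlayerCharacter only prints a red "DETECTED" message.
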(event OnComponentBeginOverlap(Trigger)
  (params (OverlappedComponent :type Primitive%20Component%20Object%20Reference) (OtherActor :type Actor%20Object%20Reference) (OtherComp :type Primitive%20Component%20Object%20Reference) (OtherBodyIndex :type Integer) (bFromSweep :type Boolean) (SweepResult :type Hit%20Result%20Structure%20%28by%20ref%29))
  ;[1 1 1] Detection
  (Utilities|Casting|CastToCore_PlayerCharacter OtherActor)
  (Development|PrintString "DETECTED" true true "(R=1.000000,G=0.088542,B=0.088542,A=1.000000)"))

(event EventTick
  (params (DeltaSeconds :type Float%20%28single-precision%29))
  (bind _travelpath (Variables|Default|GetTravelPath))
  (if (Variables|Default|GetHasLooped)
    (Variables|Default|SetCurrentDistanceAlongSpline 0.0)
    (Variables|Default|SetHasLooped false)
    (else
      (bind _output_get (Variables|Default|SetCurrentDistanceAlongSpline (Math|Interpolation|FInterptoConstant (Variables|Default|GetCurrentDistanceAlongSpline) (Spline|GetSplineLength (Variables|Default|GetTravelPath)) DeltaSeconds (Variables|Default|GetSpeed))))
      (Transformation|SetWorldLocation (Variables|Default|GetStaticMesh) (Spline|GetLocationatDistanceAlongSpline _travelpath _output_get "World") false false)
      (Transformation|SetWorldRotation (Variables|Default|GetStaticMesh) (Spline|GetRotationatDistanceAlongSpline _travelpath _output_get "Local") false false)
      (if (>= (Variables|Default|GetCurrentDistanceAlongSpline) (Spline|GetSplineLength (Variables|Default|GetTravelPath)))
        (Variables|Default|SetHasLooped true)))))

(fn ConstructionScript)