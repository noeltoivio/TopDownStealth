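; BP_SleepingGuard is an interactable sleeping guard from whom the player takes the blue keycard.
; Overlap on its Trigger shows or hides the Etext prompt and enables or disables input on the actor for the player character.
; Pressing E runs once, destroying the Keycard component, setting HasKeycard on Core_GameInstance and printing an acquisition message.
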(event OnComponentBeginOverlap(Trigger)
  (params (OverlappedComponent :type Primitive%20Component%20Object%20Reference) (OtherActor :type Actor%20Object%20Reference) (OtherComp :type Primitive%20Component%20Object%20Reference) (OtherBodyIndex :type Integer) (bFromSweep :type Boolean) (SweepResult :type Hit%20Result%20Structure%20%28by%20ref%29))
  (Utilities|Casting|CastToCore_PlayerCharacter OtherActor)
  (Input|EnableInput (Game|GetPlayerController 0))
  (Rendering|SetVisibility (Variables|Default|GetEtext) true false))

(event OnComponentEndOverlap(Trigger)
  (params (OverlappedComponent :type Primitive%20Component%20Object%20Reference) (OtherActor :type Actor%20Object%20Reference) (OtherComp :type Primitive%20Component%20Object%20Reference) (OtherBodyIndex :type Integer))
  (Utilities|Casting|CastToCore_PlayerCharacter OtherActor)
  (Input|DisableInput (Game|GetPlayerController 0))
  (Rendering|SetVisibility (Variables|Default|GetEtext) false false))

(event EventBeginPlay
  (Rendering|SetVisibility (Variables|Default|GetEtext) false false))

(event Input|ActionEvents|InputActionE
  (params (Key :type Key%20Structure))
  (:Pressed
    (Utilities|FlowControl|DoOnce false
      (:Completed
        (Components|DestroyComponent (Variables|Default|GetKeycard))
        (bind _ascore_game_instance (Utilities|Casting|CastToCore_GameInstance (Game|GetGameInstance)))
        (Variables|/Game/Root_NT/Core/Framework/Core_GameInstance.Core_GameInstance_C|SetHasKeycard _ascore_game_instance true)
        (Development|PrintString "Blue Keycard Aquired")))))

(fn ConstructionScript)