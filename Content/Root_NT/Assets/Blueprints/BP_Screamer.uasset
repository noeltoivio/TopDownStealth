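; BP_Screamer is a one-shot trigger that moves a static mesh, reveals text and alerts guards.
; At BeginPlay it hides the text and converts TargetPos from an offset to a world position.
; Player overlap with the trigger shows the text and, only the first time, runs the FreakOut timeline to lerp the mesh to that target.
; When the timeline finishes, every guard in ListeningGuards starts walking.
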(event OnComponentBeginOverlap(Trigger)
  (params (OverlappedComponent :type Primitive%20Component%20Object%20Reference) (OtherActor :type Actor%20Object%20Reference) (OtherComp :type Primitive%20Component%20Object%20Reference) (OtherBodyIndex :type Integer) (bFromSweep :type Boolean) (SweepResult :type Hit%20Result%20Structure%20%28by%20ref%29))
  (Utilities|Casting|CastToCore_PlayerCharacter OtherActor)
  (Rendering|SetVisibility (Variables|Default|GetTextRender) true false)
  (Utilities|FlowControl|DoOnce false
    (:Completed
      (bind _newtrack_0 (Timeline|FreakOut PlayFromStart)
        (:Update
          (Transformation|SetWorldLocation (Variables|Default|GetStaticMesh) (Math|Vector|Lerp(Vector) (Variables|Default|GetStartPos) (Variables|Default|GetTargetPos) _newtrack_0) false false))
        (:Finished
          (for _array_element (Variables|Default|GetListeningGuards)
            (Default|StartWalking _array_element)))))))

(event EventBeginPlay
  (bind _staticmesh (Variables|Default|GetStaticMesh))
  (bind _returnvalue (Transformation|GetWorldLocation _staticmesh))
  (Variables|Default|SetStartPos _returnvalue)
  (Variables|Default|SetTargetPos (+ (Variables|Default|GetTargetPos) _returnvalue))
  (Rendering|SetVisibility (Variables|Default|GetTextRender) false false))

(fn ConstructionScript)